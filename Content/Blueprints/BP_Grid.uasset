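; BP_Grid handles tile animations for a match-style puzzle grid: swapping, dropping down and enlarging combos.
; Each event plays a Timeline that lerps tile locations or scales tiles in X and Z with Y at zero.
; Swaps choose between valid and non-valid curves based on IsMoveCombo.
; Each Timeline calls a finished callback defined outside these graphs, leaving grid logic elsewhere.
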(event EventBeginPlay)

(event Collision|EventActorBeginOverlap
  (params (OtherActor :type Actor%20Object%20Reference)))

(event EventTick
  (params (DeltaSeconds :type Float%20%28single-precision%29)))

(event EventDropdownTiles
  (params (tiles :type Array%20of%20Tile%20Dropdown%20Data%20Structures))
  ;[1 1 1] DropdownTiles
  (bind _dropdowntrack (Timeline|Timeline_DropdownTiles PlayFromStart)
    (:Update
      (for _array_element tiles
        (Transformation|SetActorLocation (.Tile (Utilities|Struct|BreakTileDropdownData _array_element)) (Math|Vector|Lerp(Vector) (.StartingPosition (Utilities|Struct|BreakTileDropdownData _array_element)) (.DestinationPosition (Utilities|Struct|BreakTileDropdownData _array_element)) _dropdowntrack) false false)))
    (:Finished
      (Class|Grid|OnDropdownFinished))))

(event EventEnlargeComboTiles
  (params (tiles :type Array%20of%20Tile%20Object%20References))
  (bind _enlargetrack (Timeline|Timeline_EnlargeTiles PlayFromStart)
    (:Update
      (for _array_element tiles
        (Transformation|SetActorScale3D _array_element (Math|Vector|MakeVector _enlargetrack 0.0 _enlargetrack))))
    (:Finished
      (Class|Grid|OnEnlargeTilesFinished))))

(event EventSwapTiles
  (params (first :type Tile%20Object%20Reference) (second :type Tile%20Object%20Reference) (isMoveCombo :type Boolean))
  ;[1 1 1] Swap Tiles
  (Variables|Default|SetFirstTilePosition (Transformation|GetActorLocation first))
  (Variables|Default|SetSecondTilePosition (Transformation|GetActorLocation second))
  (bind (_direction _swaptilesvalidtrack _swaptilesnonvalidtrack) (Timeline|Timeline_SwapTiles PlayFromStart)
    (:Update
      (Transformation|SetActorLocation first (Math|Vector|Lerp(Vector) (Variables|Default|GetFirstTilePosition) (Variables|Default|GetSecondTilePosition) (Math|Float|SelectFloat _swaptilesvalidtrack _swaptilesnonvalidtrack isMoveCombo)) false false)
      (Transformation|SetActorLocation second (Math|Vector|Lerp(Vector) (Variables|Default|GetSecondTilePosition) (Variables|Default|GetFirstTilePosition) (Math|Float|SelectFloat _swaptilesvalidtrack _swaptilesnonvalidtrack isMoveCombo)) false false))
    (:Finished
      (Class|Grid|OnSwapTilesFinished isMoveCombo))))

(fn ConstructionScript)